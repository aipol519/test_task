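; A clickable world button actor that displays a number and spawns a turtle from a referenced turtle hole.
; On BeginPlay it passes its ButtonNumber to the NumberWidget hosted in its world widget component.
; Clicking the button mesh plays a one-shot press animation and, if the TurtleHoleRef is valid, calls SpawnTurtle on it.
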(event `self.ReceiveBeginPlay`
  (bind _asnumber_widget (cast `/Game/Widgets/NumberWidget` (`WidgetComponent.GetWidget` (`self.NumberWorldWidget`))))
  (`/Game/Widgets/NumberWidget.SetTextNumber` _asnumber_widget (`self.ButtonNumber`)))

(event `self.ButtonMesh.OnClicked`
  (params (TouchedComponent :type "PrimitiveComponent Object Reference") (ButtonPressed :type "Key Structure"))
  (bind _turtleholeref (`self.TurtleHoleRef`))
  (`SkeletalMeshComponent.PlayAnimation` (`self.ButtonMesh`) "/Game/Meshes/button/button_Anim.button_Anim" false)
  (if (`KismetSystemLibrary.IsValid` _turtleholeref)
    (`/Game/Blueprints/TurtleHoleBlueprint.SpawnTurtle` _turtleholeref)))

(fn `UserConstructionScript`)