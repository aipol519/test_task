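; TurtleHoleBlueprint is a hole actor that spawns an AI turtle and gives it a destination.
; SpawnTurtle checks that TurtleClass is valid, then plays an attenuated spawn sound and a particle effect before spawning the AI pawn at TurtleSpawnPoint.
; The spawned TurtleBlueprint receives TurtleTargetPoint's world location as its TargetLocation.
; Nothing in this graph calls SpawnTurtle.
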(fn `SpawnTurtle`
  (bind _turtlespawnpoint (`self.TurtleSpawnPoint`))
  (if (`KismetSystemLibrary.IsValidClass` (`self.TurtleClass`))
    (`GameplayStatics.PlaySoundAtLocation` "/Game/Sounds/turtle_spawn.turtle_spawn" (`self.K2_GetActorLocation`) (struct) 1.0 1.0 0.0 "/Game/Sounds/SoundAttenuation.SoundAttenuation" null null)
    (`GameplayStatics.SpawnEmitterAtLocation` "/Game/Particles/spawn_particle.spawn_particle" (`SceneComponent.K2_GetComponentLocation` (`self.TurtleSpawnPoint`)))
    (bind _returnvalue (`AIBlueprintHelperLibrary.SpawnAIFromClass` (`self.TurtleClass`) null (`SceneComponent.K2_GetComponentLocation` _turtlespawnpoint) (`SceneComponent.K2_GetComponentRotation` _turtlespawnpoint) false null))
    (bind _asturtle_blueprint (cast `/Game/Blueprints/Turtles/TurtleBlueprint` _returnvalue))
    (set `/Game/Blueprints/Turtles/TurtleBlueprint.TargetLocation` (`SceneComponent.K2_GetComponentLocation` (`self.TurtleTargetPoint`)) _asturtle_blueprint)))

(fn `UserConstructionScript`)