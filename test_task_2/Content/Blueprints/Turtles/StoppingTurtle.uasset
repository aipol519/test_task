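; Turtle variant that travels to its target location in a stop-and-go rhythm, alternating one second of movement with one second of pause.
; StartMove and StopMoving re-arm each other through timers by function name, issuing or halting the AI move while toggling step sound, animation and dust.
; An audio component validity check gates starting the effects.
; A successful move completion runs the parent handler, then clears the pending stop timer to end the cycle.
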(event `self.OnMoveCompleted`
  (params (RequestID :type "AIRequestID Structure") (Result :type "EPathFollowingResult Enum" :default "Success"))
  (`parent.OnMoveCompleted` RequestID Result)
  (if (`|EnumEquality` Result "Success")
    (`KismetSystemLibrary.K2_ClearTimer` self "StopMoving")))

(fn `StartMove`
  (`KismetSystemLibrary.K2_SetTimer` self "StopMoving" 1.0)
  (if (not (`KismetSystemLibrary.IsValid` (`self.TurtleAudioComponent`)))
    (bind _returnvalue (`GameplayStatics.SpawnSoundAttached` "/Game/Sounds/turtle_step.turtle_step" (`self.DefaultSceneRoot`) "None" (0.0 0.0 0.0) (struct) "KeepRelativeOffset" false 1.0 1.0 0.0 "/Game/Sounds/SoundAttenuation.SoundAttenuation" null))
    (set `self.TurtleAudioComponent` _returnvalue)
    (`SkeletalMeshComponent.PlayAnimation` (`self.TurtleMesh`) "/Game/Meshes/turtle/turtle_Anim.turtle_Anim" true)
    (`ActorComponent.Activate` (`self.StepDustEmitter`) false))
  (`AIController.MoveToLocation` (`AIBlueprintHelperLibrary.GetAIController` self) (`self.TargetLocation`) 1.0 false true false true null true))

(fn `StopMoving`
  (`KismetSystemLibrary.K2_SetTimer` self "StartMove" 1.0)
  (`AudioComponent.Stop` (`self.TurtleAudioComponent`))
  (`SkeletalMeshComponent.Stop` (`self.TurtleMesh`))
  (`ActorComponent.Deactivate` (`self.StepDustEmitter`))
  (`Controller.StopMovement` (`self.GetController`)))

(fn `UserConstructionScript`
  (`parent.UserConstructionScript`))