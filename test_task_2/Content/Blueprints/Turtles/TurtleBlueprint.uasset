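; Base turtle actor that starts moving shortly after spawn and celebrates when its AI move reaches the goal.
; BeginPlay binds to the AI controller's move-completed event, then after a delay starts the step audio, walk animation, dust and StartMove.
; StartMove is an empty function here, presumably for child Blueprints to override.
; A successful move clears any StartMove timer, stops those effects and plays goal sound and particles at TargetLocation.
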(event `self.ReceiveBeginPlay`
  (add `AIController.ReceiveMoveCompleted` (`AIBlueprintHelperLibrary.GetAIController` self) (delegate `OnMoveCompleted`))
  (`KismetSystemLibrary.Delay` 1.0)
  (bind _returnvalue (`GameplayStatics.SpawnSoundAttached` "/Game/Sounds/turtle_step.turtle_step" (`self.DefaultSceneRoot`) "None" (0.0 0.0 0.0) (struct) "KeepRelativeOffset" false 1.0 1.0 0.0 "/Game/Sounds/SoundAttenuation.SoundAttenuation" null))
  (set `self.TurtleAudioComponent` _returnvalue)
  (`self.OnSpawned`))

(event `OnMoveCompleted`
  (params (RequestID :type "AIRequestID Structure") (Result :type "EPathFollowingResult Enum" :default "Success"))
  (bind _targetlocation (`self.TargetLocation`))
  (if (`|EnumEquality` Result "Success")
    (`KismetSystemLibrary.K2_ClearTimer` self "StartMove")
    (`AudioComponent.Stop` (`self.TurtleAudioComponent`))
    (`SkeletalMeshComponent.Stop` (`self.TurtleMesh`))
    (`ActorComponent.Deactivate` (`self.StepDustEmitter`))
    (`GameplayStatics.PlaySoundAtLocation` "/Game/Sounds/turtle_goal_reached.turtle_goal_reached" _targetlocation (struct) 1.0 1.0 0.0 "/Game/Sounds/SoundAttenuation.SoundAttenuation" null null)
    (`GameplayStatics.SpawnEmitterAtLocation` "/Game/Particles/goal_particle.goal_particle" _targetlocation)))

(event `OnSpawned`
  (`SkeletalMeshComponent.PlayAnimation` (`self.TurtleMesh`) "/Game/Meshes/turtle/turtle_Anim.turtle_Anim" true)
  (`ActorComponent.Activate` (`self.StepDustEmitter`) false)
  (`self.StartMove`))

(fn `StartMove`)

(fn `UserConstructionScript`)