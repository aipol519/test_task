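; Turtle variant that advances toward its target in a back-and-forth pattern, periodically retreating toward where it began.
; StartMove and MoveBackward schedule each other by timer, alternating one second of AI movement toward TargetLocation with half a second toward the StartLocation saved at BeginPlay.
; A successful move completion clears any pending MoveBackward timer, so reaching the target stops the cycle.
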(event `self.ReceiveBeginPlay`
  (`parent.ReceiveBeginPlay`)
  (set `self.StartLocation` (`self.K2_GetActorLocation` self)))

(event `self.OnMoveCompleted`
  (params (RequestID :type "AIRequestID Structure") (Result :type "EPathFollowingResult Enum" :default "Success"))
  (`parent.OnMoveCompleted` RequestID Result)
  (if (`|EnumEquality` Result "Success")
    (`KismetSystemLibrary.K2_ClearTimer` self "MoveBackward")))

(fn `MoveBackward`
  (`KismetSystemLibrary.K2_SetTimer` self "StartMove" 0.5)
  (`AIController.MoveToLocation` (`AIBlueprintHelperLibrary.GetAIController` self) (`self.StartLocation`) 1.0 false true false true null true))

(fn `StartMove`
  (`KismetSystemLibrary.K2_SetTimer` self "MoveBackward" 1.0)
  (`AIController.MoveToLocation` (`AIBlueprintHelperLibrary.GetAIController` self) (`self.TargetLocation`) 1.0 false true false true null true))

(fn `UserConstructionScript`
  (`parent.UserConstructionScript`))